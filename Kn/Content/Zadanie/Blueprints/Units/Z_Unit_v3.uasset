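; Selectable RTS-style unit that automatically fires on targetable actors within range and takes move orders.
; Detection sphere overlaps and destroy bindings maintain a target list; when the current target becomes invalid, another is taken.
; A looping timer spawns bullets aimed at the target and is cleared when none remain.
; Selection binds the controller's deselect and move commands, tints a dynamic material, and moves run through AI MoveTo, ending any previous task.
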(event OnComponentBeginOverlap(Detection_Radius)
  (params (OverlappedComponent :type Primitive%20Component%20Object%20Reference) (OtherActor :type Actor%20Object%20Reference) (OtherComp :type Primitive%20Component%20Object%20Reference) (OtherBodyIndex :type Integer) (bFromSweep :type Boolean) (SweepResult :type Hit%20Result%20Structure%20%28by%20ref%29))
  ;[1 1 1] Manage set and on destroy event binding
  (Utilities|Casting|CastToZ_Targetable OtherActor)
  (Utilities|Set|Add (Variables|Default|GetList_Of_Targets) OtherActor)
  (Game|AssignOnDestroyed OtherActor (delegate Custom|Remove_Target_PostMoretem))
  ;[1 1 1] Update IF we fire and on what
  (CallFunction|UpdateTargets))

(event OnComponentEndOverlap(Detection_Radius)
  (params (OverlappedComponent :type Primitive%20Component%20Object%20Reference) (OtherActor :type Actor%20Object%20Reference) (OtherComp :type Primitive%20Component%20Object%20Reference) (OtherBodyIndex :type Integer))
  ;[1 1 1] Manage set and on destroy event binding
  (Utilities|Casting|CastToZ_Targetable OtherActor)
  (Utilities|Set|Remove (Variables|Default|GetList_Of_Targets) OtherActor)
  (Game|UnbindEventfromOnDestroyed OtherActor (delegate Custom|Remove_Target_PostMoretem))
  ;[1 1 1] Update IF we fire and on what
  (Utilities|FlowControl|Sequence
    (:then_0
      ;[1 1 1] Check if CURRENT target will be valid or we take next target
      (Utilities|IsValid (Variables|Default|GetTarget)
        (:Is%20Valid
          (Variables|Default|SetIs_Target_Valid (!= OtherActor (Variables|Default|GetTarget))))))
    (:then_1
      (CallFunction|UpdateTargets))))

(event Custom|Remove_Target_PostMoretem
  (params (DestroyedActor :type Actor%20Object%20Reference))
  ;[1 1 1] Manage set and on destroy event binding
  (Utilities|Casting|CastToZ_Targetable DestroyedActor)
  (Utilities|Set|Remove (Variables|Default|GetList_Of_Targets) DestroyedActor)
  (Game|UnbindEventfromOnDestroyed DestroyedActor (delegate Custom|Remove_Target_PostMoretem))
  ;[1 1 1] Update IF we fire and on what
  (Utilities|FlowControl|Sequence
    (:then_0
      ;[1 1 1] Check if CURRENT target will be valid or we take next target
      (Utilities|IsValid (Variables|Default|GetTarget)
        (:Is%20Valid
          (Variables|Default|SetIs_Target_Valid (!= DestroyedActor (Variables|Default|GetTarget))))))
    (:then_1
      (CallFunction|UpdateTargets))))

(event Custom|Update_Targets
  (if (not (Variables|Default|GetIs_Target_Valid))
    (if (< 0 (Utilities|Set|Length (Variables|Default|GetList_Of_Targets))) ; do we have more than 0 possible targets?
      (bind _result (Utilities|Set|ToArray (Variables|Default|GetList_Of_Targets)))
      (bind _output_get (Variables|Default|SetTarget (Utilities|Array|Get(acopy) _result)))
      (Utilities|Set|Remove (Variables|Default|GetList_Of_Targets) _output_get)
      (Variables|Default|SetIs_Target_Valid true)
      (if (not (Utilities|Time|IsValidTimerHandle (Variables|Default|GetFire_Timer)))
        (bind _returnvalue (Utilities|Time|SetTimerbyEvent (delegate Custom|Attack_Clock) (Variables|Default|GetFire_Rate) true))
        (Variables|Default|SetFire_Timer _returnvalue))
      (else
        (Utilities|Time|ClearandInvalidateTimerbyHandle (Variables|Default|GetFire_Timer))))))

(event Custom|Attack_Clock
  (bind _returnvalue (Transformation|GetActorTransform))
  (bind _target (Variables|Default|GetTarget))
  (Utilities|String|LogString (Utilities|String|Append (Utilities|GetDisplayName self) " attacks " (Utilities|GetDisplayName (Variables|Default|GetTarget))))
  (Game|SpawnActorfromClass "/Game/Zadanie/Blueprints/Bullets/Z_Bullet.Z_Bullet_C" (Math|Transform|MakeTransform (.location _returnvalue) (Math|Rotator|FindLookatRotation (.location _returnvalue) (.location (Transformation|GetActorTransform _target))) "0.200000,0.200000,0.200000") "Undefined" 0 _target self))

(event Custom|Command_Deselect
  (params (UnbindTo :type Z%20Player%20Controler%20Object%20Reference))
  ;[1 1 1] Bind and unbind controls from controler as well as colors
  (Utilities|FlowControl|Sequence
    (:then_0
      (EventDispatchers|UnbindEventfromCommandDeselect UnbindTo (delegate Custom|Command_Deselect)))
    (:then_1
      (EventDispatchers|UnbindEventfromCommandMove UnbindTo (delegate Custom|Command_Move)))
    (:then_2
      (CallFunction|SetColorSelected false))))

(event Custom|Command_Move
  (params (Location :type Vector))
  (Utilities|IsValid (Variables|Default|GetAsync_Task_Move_To_Location) ; tak naprawdę zadanie poruszania się powinno być też zatrzymane\n gdy aktor nie może się bardziel zlbiżyć do celu. Przykład takiej\n implementacji (z wykorzystaniem dynamicznych przeszkód dla navmesh)\n jest w pracy którą wcześniej wysłałem
    (:Is%20Valid
      (GameplayTasks|EndTask (Variables|Default|GetAsync_Task_Move_To_Location)))
    (:Is%20Not%20Valid
      _))
  (bind _asynctaskproxy (AI|AIMoveTo (AI|GetAIController self) Location 0 -1.0 "Default" "Enable" true true)
    (:then
      (Variables|Default|SetAsync_Task_Move_To_Location _asynctaskproxy))))

(event EventBeginPlay
  (bind _returnvalue (Rendering|Material|CreateDynamicMaterialInstance "/Game/Zadanie/Materials/Flat_Material.Flat_Material" "None" "None" :!class /Script/Engine.KismetMaterialLibrary))
  (bind _output_get (Variables|Default|SetUnit_Color_Material _returnvalue))
  (Rendering|Material|SetMaterial (Variables|Default|GetShape) 0 _output_get))

(event Collision|EventActorBeginOverlap
  (params (OtherActor :type Actor%20Object%20Reference)))

(event EventTick
  (params (DeltaSeconds :type Float%20%28single-precision%29)))

(event EventSelectableSelect
  (params (BindTo :type Z%20Player%20Controler%20Object%20Reference))
  ;[1 1 1] Bind and unbind controls from controler as well as colors
  (Utilities|FlowControl|Sequence
    (:then_0
      (EventDispatchers|BindEventtoCommandDeselect BindTo (delegate Custom|Command_Deselect)))
    (:then_1
      (EventDispatchers|BindEventtoCommandMove BindTo (delegate Custom|Command_Move)))
    (:then_2
      (CallFunction|SetColorSelected true))))

(fn ConstructionScript
  (Components|Sphere|SetSphereRadius (Variables|Default|GetDetection_Radius) (Variables|Default|GetRange) true))

(fn SetColorSelected
  (params (IsSelected? :type Boolean))
  (bind _unit_color_material (Variables|Default|GetUnit_Color_Material))
  (Rendering|Material|SetVectorParameterValue _unit_color_material "Color" (Math|Color|SelectColor "(R=0.000000,G=1.000000,B=0.000000,A=1.000000)" "(R=1.000000,G=1.000000,B=1.000000,A=1.000000)" IsSelected?) :!class /Script/Engine.MaterialInstanceDynamic)
  (Rendering|Material|SetScalarParameterValue _unit_color_material "Emissive" (Math|Float|SelectFloat 1e+01 0.0 IsSelected?) :!class /Script/Engine.MaterialInstanceDynamic))