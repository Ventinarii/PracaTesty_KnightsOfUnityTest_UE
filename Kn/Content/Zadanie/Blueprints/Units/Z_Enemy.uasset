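; Enemy unit that chases whoever damages it and destroys itself along with any player unit it reaches.
; On TargetableTakeDamage, if no valid attacker is stored, it saves WhoFired and starts an AI MoveTo with continuous goal tracking, ending any previous task.
; Interaction_Radius overlap casts directly to Z_Unit_v3, a deliberate shortcut instead of an interface, then destroys both actors.
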(event OnComponentBeginOverlap(Interaction_Radius)
  (params (OverlappedComponent :type Primitive%20Component%20Object%20Reference) (OtherActor :type Actor%20Object%20Reference) (OtherComp :type Primitive%20Component%20Object%20Reference) (OtherBodyIndex :type Integer) (bFromSweep :type Boolean) (SweepResult :type Hit%20Result%20Structure%20%28by%20ref%29))
  (bind _asz_unit_v_3 (Utilities|Casting|CastToZ_Unit_v3 OtherActor)) ; Tu tak naprawdę powinien być interfejs ale \njako że jest tylko jedna klasa którą steruje \ngracz to zostało to uproszczone
  (Actor|DestroyActor _asz_unit_v_3)
  (Actor|DestroyActor self))

(event EventBeginPlay)

(event Collision|EventActorBeginOverlap
  (params (OtherActor :type Actor%20Object%20Reference)))

(event EventTick
  (params (DeltaSeconds :type Float%20%28single-precision%29)))

(event EventTargetableTakeDamage
  (params (Who_Fired :type Actor%20Object%20Reference))
  (Utilities|IsValid (Variables|Default|GetWho%20Fired)
    (:Is%20Not%20Valid
      (Variables|Default|SetWho%20Fired Who_Fired)
      (Utilities|IsValid (stale _asynctaskproxy)
        (:Is%20Valid
          (GameplayTasks|EndTask (stale _asynctaskproxy)))
        (:Is%20Not%20Valid
          _))
      (bind _asynctaskproxy (AI|AIMoveTo (AI|GetAIController self) "0, 0, 0" Who_Fired -1.0 "Default" "Enable" true true true)))))

(fn ConstructionScript)