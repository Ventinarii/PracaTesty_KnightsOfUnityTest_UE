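; Player controller for RTS-style play: moves camera and pawn, selects units and issues move orders.
; Directional actions feed HandleInput, which accumulates separate camera and pawn axis vectors by adding or cancelling unit vectors on press/release, then broadcasts them.
; Cursor traces select a Z_Selectable or start a zone drag, updated on Tick through a dispatcher.
; Select_Zone_Return selects returned actors; Order_Unit broadcasts the move location.
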(event Custom|Select_Zone_Return
  (params (Actors :type Array%20of%20Actor%20Object%20References))
  (for _array_element Actors
    (bind _asz_selectable (Utilities|Casting|CastToZ_Selectable _array_element))
    (Default|SelectableSelect _asz_selectable self)))

(event EventTick
  (params (DeltaSeconds :type Float%20%28single-precision%29))
  (Utilities|FlowControl|Sequence
    (:then_0
      (if (Variables|Default|GetSelect_Zone_In_Progress)
        (Default|CallSfxSelectZone (Variables|Default|GetSelect_Zone_From) (.location (.HitResult (Game|Player|GetHitResultUnderCursorbyChannel self "TraceTypeQuery2" false))) true)))))

(event Input|ActionEvents|InputActionPawn_Up
  (params (Key :type Key%20Structure :default "None"))
  (bind _returnvalue (Class|KismetSystemLibrary|MakeLiteralBool false))
  (:Pressed
    (CallFunction|HandleInput true true true _returnvalue))
  (:Released
    (CallFunction|HandleInput true true false _returnvalue)))

(event Input|ActionEvents|InputActionCamera_Up
  (params (Key :type Key%20Structure :default "None"))
  (bind _returnvalue (Class|KismetSystemLibrary|MakeLiteralBool true))
  (:Pressed
    (CallFunction|HandleInput true true true _returnvalue))
  (:Released
    (CallFunction|HandleInput true true false _returnvalue)))

(event Input|ActionEvents|InputActionSelect_Unit
  (params (Key :type Key%20Structure :default "None"))
  (bind _self self)
  (bind _hitresult (Game|Player|GetHitResultUnderCursorbyChannel _self "TraceTypeQuery2" false))
  (:Pressed
    (Default|CallCommandDeselect self)
    (bind _asz_selectable (Utilities|Casting|CastToZ_Selectable (.hitactor _hitresult))
      (:then
        (Default|SelectableSelect _asz_selectable self))
      (:CastFailed
        (bind _output_get (Variables|Default|SetSelect_Zone_From (.location _hitresult)))
        (Variables|Default|SetSelect_Zone_In_Progress true))))
  (:Released
    (Variables|Default|SetSelect_Zone_In_Progress false)
    (Default|CallSfxSelectZone _output_get (.location _hitresult) false)))

(event Input|ActionEvents|InputActionOrder_Unit
  (params (Key :type Key%20Structure :default "None"))
  (:Pressed
    (Default|CallCommandMove (.location (.HitResult (Game|Player|GetHitResultUnderCursorbyChannel self "TraceTypeQuery2" false))))))

(event Input|ActionEvents|InputActionCamera_Left
  (params (Key :type Key%20Structure :default "None"))
  (bind _returnvalue (Class|KismetSystemLibrary|MakeLiteralBool true))
  (:Pressed
    (CallFunction|HandleInput false false true _returnvalue))
  (:Released
    (CallFunction|HandleInput false false false _returnvalue)))

(event Input|ActionEvents|InputActionPawn_Right
  (params (Key :type Key%20Structure :default "None"))
  (bind _returnvalue (Class|KismetSystemLibrary|MakeLiteralBool false))
  (:Pressed
    (CallFunction|HandleInput false true true _returnvalue))
  (:Released
    (CallFunction|HandleInput false true false _returnvalue)))

(event Input|ActionEvents|InputActionCamera_Down
  (params (Key :type Key%20Structure :default "None"))
  (bind _returnvalue (Class|KismetSystemLibrary|MakeLiteralBool true))
  (:Pressed
    (CallFunction|HandleInput true false true _returnvalue))
  (:Released
    (CallFunction|HandleInput true false false _returnvalue)))

(event Input|ActionEvents|InputActionCamera_Right
  (params (Key :type Key%20Structure :default "None"))
  (bind _returnvalue (Class|KismetSystemLibrary|MakeLiteralBool true))
  (:Pressed
    (CallFunction|HandleInput false true true _returnvalue))
  (:Released
    (CallFunction|HandleInput false true false _returnvalue)))

(event Input|ActionEvents|InputActionPawn_Down
  (params (Key :type Key%20Structure :default "None"))
  (bind _returnvalue (Class|KismetSystemLibrary|MakeLiteralBool false))
  (:Pressed
    (CallFunction|HandleInput true false true _returnvalue))
  (:Released
    (CallFunction|HandleInput true false false _returnvalue)))

(event Input|ActionEvents|InputActionPawn_Left
  (params (Key :type Key%20Structure :default "None"))
  (bind _returnvalue (Class|KismetSystemLibrary|MakeLiteralBool false))
  (:Pressed
    (CallFunction|HandleInput false false true _returnvalue))
  (:Released
    (CallFunction|HandleInput false false false _returnvalue)))

(fn ConstructionScript)

(fn HandleInput
  (params (X_Axis? :type Boolean) (Positive? :type Boolean) (Pressed? :type Boolean) (Camera_Controll? :type Boolean))
  (bind _returnvalue (Math|Vector|SelectVector "1.000000, 0, 0" "0,1.000000, 0" X_Axis?))
  (if Camera_Controll?
    (bind _output_get (Variables|Default|SetMovment_Axes_Camera_Dispatcher (+ (Math|Vector|SelectVector (Variables|Default|GetMovment_Axes_Camera_Dispatcher) (Variables|Default|GetMovment_Axes_Pawn) Camera_Controll?) (Math|Vector|SelectVector (* _returnvalue (Math|Float|MakeLiteralFloat -1.0)) _returnvalue (Class|KismetMathLibrary|XORBoolean Positive? Pressed?)))))
    (Default|CallMovementAxesCameraDispatcher _output_get)
    (else
      (bind _output_get_2 (Variables|Default|SetMovment_Axes_Pawn (+ (Math|Vector|SelectVector (Variables|Default|GetMovment_Axes_Camera_Dispatcher) (Variables|Default|GetMovment_Axes_Pawn) Camera_Controll?) (Math|Vector|SelectVector (* _returnvalue (Math|Float|MakeLiteralFloat -1.0)) _returnvalue (Class|KismetMathLibrary|XORBoolean Positive? Pressed?)))))
      (Default|CallMovmentAxesPawnDispatcher _output_get_2))))