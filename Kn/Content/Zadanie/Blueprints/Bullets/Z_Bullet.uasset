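; Z_Bullet is a homing projectile that seeks a single assigned Target and damages it on contact.
; At BeginPlay it sets the ProjectileMovement homing component to the Target's root component.
; Overlaps with other actors are ignored; on overlapping the Target it casts to Z_Targetable, calls TargetableTakeDamage with its Instigator, then destroys itself.
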(event EventBeginPlay
  (Variables|/Script/Engine.ProjectileMovementComponent|SetHomingTargetComponent (Variables|Default|GetProjectileMovement) (Variables|/Script/Engine.Actor|GetRootComponent (Variables|Default|GetTarget))))

(event Collision|EventActorBeginOverlap
  (params (OtherActor :type Actor%20Object%20Reference))
  (if (== OtherActor (Variables|Default|GetTarget))
    (Utilities|FlowControl|Sequence
      (:then_0
        (bind _asz_targetable (Utilities|Casting|CastToZ_Targetable OtherActor))
        (Default|TargetableTakeDamage _asz_targetable (Variables|Actor|GetInstigator)))
      (:then_1
        (Actor|DestroyActor)))))

(event EventTick
  (params (DeltaSeconds :type Float%20%28single-precision%29)))

(fn ConstructionScript)