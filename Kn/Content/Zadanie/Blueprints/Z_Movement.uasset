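; Z_Movement is a movement component that slides its owner's root component according to player input axes.
; On BeginPlay it subscribes to either the camera or pawn axes dispatcher on Z_Player_Controler, chosen by the IsOnCamera flag, so one component serves both cases.
; The dispatcher updates the stored axes, and Tick applies them as a swept world offset scaled by speed and delta time.
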(event Custom|UpdateAxes
  (params (Axes :type Vector))
  (Variables|Default|SetMovment_Axes Axes))

(event EventBeginPlay
  (Variables|Default|SetRoot%20Component (Variables|/Script/Engine.Actor|GetRootComponent (Components|GetOwner)))
  (bind _asz_player_controler (Utilities|Casting|CastToZ_Player_Controler (Game|GetPlayerController 0)))
  (bind _output_get (Variables|Default|SetAs%20Z%20Player%20Controler _asz_player_controler))
  (if (Variables|Default|GetIsOnCamera)
    (EventDispatchers|BindEventtoMovementAxesCameraDispatcher _output_get (delegate Custom|UpdateAxes))
    (else
      (EventDispatchers|BindEventtoMovmentAxesPawnDispatcher _output_get (delegate Custom|UpdateAxes)))))

(event EventTick
  (params (DeltaSeconds :type Float%20%28single-precision%29))
  (Transformation|AddWorldOffset (Variables|Default|GetRoot%20Component) (* (Variables|Default|GetMovment_Axes) (Variables|Default|GetMovement_Speed) DeltaSeconds) true false))