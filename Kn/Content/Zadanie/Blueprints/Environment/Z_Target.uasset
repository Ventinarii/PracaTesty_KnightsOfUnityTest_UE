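; Z_Target is a damageable target that displays its HP on a Z_HpBar widget.
; BeginPlay pushes the current HP from ZHealthAtributeSet to the bar, and TargetableTakeDamage calls Hit on that set, then refreshes the bar.
; This is a stopgap without the ability system.
; An unreachable GiveAbility/TryActivateAbility version remains, noted as abandoned because it created new instances instead of reusing one.
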(event EventBeginPlay
  ;[1 1 1] Rozwiązanie zastępcze bez ability system
  (bind _asz_hp_bar (Utilities|Casting|CastToZ_HpBar (UserInterface|GetWidget (Variables|Default|GetHp))))
  (Utilities|IsValid _asz_hp_bar
    (:Is%20Valid
      (Utilities|IsValid (Variables|Default|GetZ_HealthAtributeSet)
        (:Is%20Valid
          (bind _hp_ (Default|Hp% (Variables|Default|GetZ_HealthAtributeSet)))
          (Default|SetHp _asz_hp_bar _hp_))))))

(event EventTargetableTakeDamage
  (params (Who_Fired :type Actor%20Object%20Reference))
  ;[1 1 1] Rozwiązanie zastępcze bez ability system
  (Default|Hit (Variables|Default|GetZ_HealthAtributeSet))
  (Utilities|IsValid (stale EventBeginPlay _asz_hp_bar)
    (:Is%20Valid
      (Utilities|IsValid (Variables|Default|GetZ_HealthAtributeSet)
        (:Is%20Valid
          (bind _hp_ (Default|Hp% (Variables|Default|GetZ_HealthAtributeSet)))
          (Default|SetHp (stale EventBeginPlay _asz_hp_bar) _hp_))))))

(fn ConstructionScript)