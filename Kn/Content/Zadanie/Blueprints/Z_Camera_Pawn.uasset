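; Camera pawn that provides an area-selection zone, shown with a decal, for the player controller.
; On BeginPlay it binds to the controller's SfxSelectZone event, hides the decal and detaches the decal and box.
; Each event scales and centers both between two points, padded vertically to avoid height problems.
; Decal visibility follows the active flag; when selection ends, the box's overlapping actors go back via SelectZoneReturn.
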(event Custom|SelectZone
  (params (From :type Vector) (To :type Vector) (Active :type Boolean))
  (bind _returnvalue (Math|Float|MakeLiteralFloat 2.0))
  (bind _returnvalue_2 (Math|Vector|VectorUp))
  (bind _returnvalue_3 (Math|Float|MakeLiteralFloat 2e+02))
  (bind (_x _y _z) (Class|KismetMathLibrary|BreakVector3f To))
  (bind (_x_2 _y_2 _z_2) (Class|KismetMathLibrary|BreakVector3f From))
  (bind _decal (Variables|Default|GetDecal))
  (bind _returnvalue_4 (Math|Float|Min(Float) _z_2 _z))
  (bind _returnvalue_5 (Math|Float|Min(Float) _x_2 _x))
  (bind _returnvalue_6 (Math|Float|Min(Float) _y_2 _y))
  (bind _returnvalue_7 (Math|Float|Max(Float) _z_2 _z))
  (bind _returnvalue_8 (Math|Float|Max(Float) _x_2 _x))
  (bind _returnvalue_9 (Math|Float|Max(Float) _y_2 _y))
  (bind _returnvalue_10 (* _returnvalue_2 _returnvalue_3 _returnvalue))
  (bind _returnvalue_11 (Math|Vector|MakeVector _returnvalue_5 _returnvalue_6 _returnvalue_4))
  (bind _returnvalue_12 (Math|Vector|MakeVector _returnvalue_8 _returnvalue_9 _returnvalue_7))
  (bind _returnvalue_13 (+ _returnvalue_10 _returnvalue_12))
  (bind _returnvalue_14 (- _returnvalue_11 _returnvalue_10))
  (Utilities|FlowControl|Sequence
    (:then_0
      (if (Class|KismetMathLibrary|XORBoolean (Variables|/Script/Engine.SceneComponent|GetbVisible (Variables|Default|GetDecal)) Active)
        (Rendering|SetVisibility (Variables|Default|GetDecal) Active false)
        (if (not Active)
          (Default|SelectZoneReturn (stale EventBeginPlay _asz_player_controler) (Collision|GetOverlappingActors (Variables|Default|GetBox) 0 :!class /Script/Engine.PrimitiveComponent)))))
    (:then_1
      (Transformation|SetWorldScale3D _decal (/ (- _returnvalue_13 _returnvalue_14) _returnvalue_3))
      (Transformation|SetWorldLocation _decal (* (+ _returnvalue_14 _returnvalue_13) (Math|Float|MakeLiteralFloat 0.5)) true false))))

(event EventBeginPlay
  (bind _asz_player_controler (Utilities|Casting|CastToZ_Player_Controler (Game|GetPlayerController 0)))
  (EventDispatchers|BindEventtoSfxSelectZone _asz_player_controler (delegate Custom|SelectZone))
  (Rendering|SetVisibility (Variables|Default|GetDecal) false false)
  (Transformation|DetachFromComponent (Variables|Default|GetDecal) "KeepRelative" "KeepRelative" "KeepRelative" true))

(event Collision|EventActorBeginOverlap
  (params (OtherActor :type Actor%20Object%20Reference)))

(fn ConstructionScript)