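; Z_HealthAtributeSet is a health component that tracks hit points for its owning actor.
; Hit lowers CurrentHealth by one and destroys the owner once it reaches zero or below.
; Hp% returns CurrentHealth divided by MaxHealth as a fraction.
; Despite the attribute set name, it uses plain variables and functions, with no active event graph logic.
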(event EventBeginPlay)

(event EventTick
  (params (DeltaSeconds :type Float%20%28single-precision%29)))

(fn Hit
  (bind _result (Math|Float|DecrementFloat (Variables|Default|GetCurrentHealth))
    (:%20%20
      (if (<= _result 0.0)
        (Actor|DestroyActor (Components|GetOwner))))))

(fn Hp%
  (return (/ (Variables|Default|GetCurrentHealth) (Variables|Default|GetMaxHealth))))